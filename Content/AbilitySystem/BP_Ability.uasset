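; BP_Ability is an ability actor that handles casting, with an empty ActivateEffect function.
; On BeginPlay it snaps to the caster's right-hand socket, caches the player and HUD, then begins casting.
; A positive cast time shows a HUD cast bar and binds its success event; otherwise it casts immediately.
; Casting only detaches the actor in world space, while interrupting destroys it and prints a message.
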(event EventBeginPlay
  (Transformation|AttachComponentToComponent (Variables|/Script/Engine.Character|GetMesh (Variables|Default|GetCaster)) "hand_rSocket" "SnapToTarget" "SnapToTarget" "SnapToTarget" true)
  (bind _aspuzzle_platforms_character (Utilities|Casting|CastToPuzzlePlatformsCharacter (Game|GetPlayerCharacter 0)))
  (Variables|Default|SetPlayerRef _aspuzzle_platforms_character)
  (bind _aspuzzle_platforms_game_instance (Utilities|Casting|CastToPuzzlePlatformsGameInstance (Game|GetGameInstance)))
  (bind _asheads_up_display (Utilities|Casting|CastToHeadsUpDisplay (Variables|/Script/PuzzlePlatforms.PuzzlePlatformsGameInstance|GetHeadsUpDisplay _aspuzzle_platforms_game_instance)))
  (Variables|Default|SetHUD_UI _asheads_up_display)
  (CallFunction|BeginCasting))

(fn ConstructionScript)

(fn BeginCasting
  (if (> (.casttime (Variables|Default|GetAbilityDetails)) 0.0)
    (bind _castbar (Default|DisplayCastBar (Variables|Default|GetHUD_UI) self))
    (EventDispatchers|BindEventtoCastSuccessful _castbar (EventDispatchers|CreateEvent :!event CastAbility))
    (else
      (CallFunction|CastAbility))))

(fn CastAbility
  (Transformation|DetachFromActor "KeepWorld" "KeepWorld" "KeepWorld"))

(fn InterruptCast
  (Actor|DestroyActor)
  (Development|PrintString "Interrupt"))

(fn ActivateEffect)