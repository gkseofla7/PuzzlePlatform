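; BP_SoulItem is a soul pickup that flies to the player on its own after spawning.
; After a short random delay on BeginPlay, it turns off sphere physics and stores its current location.
; The MoveToPlayer timeline then lerps it from that point to the player's live position without sweeping, so it homes in on a moving target.
; When the timeline finishes it calls FinishCollectItem, with no overlap check involved.
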(event EventBeginPlay
  (Utilities|FlowControl|Delay (Math|Random|RandomFloatinRange 0.5 1.0))
  (Physics|SetSimulatePhysics (Variables|Default|GetSphereComponent) false)
  (Variables|Default|SetInitialActorLocation (Transformation|GetActorLocation))
  (bind _alpha (Timeline|MoveToPlayer Play)
    (:Update
      (Transformation|SetActorLocation (Math|Vector|Lerp(Vector) (Variables|Default|GetInitialActorLocation) (Transformation|GetActorLocation (Variables|Default|GetPlayerRef)) _alpha) false false))
    (:Finished
      (Class|SoulItem|FinishCollectItem))))

(event Collision|EventActorBeginOverlap
  (params (OtherActor :type Actor%20Object%20Reference)))

(event EventTick
  (params (DeltaSeconds :type Float%20%28single-precision%29)))

(fn ConstructionScript)