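; Auto-targeting turret that fires short bursts of bullets from twin barrels.
; Each tick it looks for the best target and, when one is valid, updates rotation and firing through functions whose bodies are not in this file.
; Fire uses a self-re-entering DoN with delays to alternate left and right shots from barrel sockets, starting a curve-driven recoil timeline for each.
; Some leftover look-at rotation logic is unconnected.
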(event EventBeginPlay
  (Class|TimelineComponent|SetFloatCurve (Variables|Default|GetRecoilTimelineL) "/Game/Turret/RecoilCurve.RecoilCurve" "Recoil")
  (Class|TimelineComponent|SetFloatCurve (Variables|Default|GetRecoilTimelineR) "/Game/Turret/RecoilCurve.RecoilCurve" "Recoil"))

(event EventFire
  (Variables|Default|SetTimeOfLastFire (Utilities|Time|GetGameTimeinSeconds))
  (Utilities|FlowControl|Sequence
    (:then_0
      (goto _label Reset))
    (:then_1
      (Utilities|FlowControl|DoN 2 :!label _label
        (:Exit
          (Game|SpawnActorfromClass "/Game/Weapons/Projectiles/BP_Bullet_Master.BP_Bullet_Master_C" (Transformation|GetSocketTransform (Variables|Default|GetStaticMeshBarrelL) "FireSocket" "RTS_World") "Undefined" 0 0)
          (Components|Timeline|PlayfromStart (Variables|Default|GetRecoilTimelineL))
          (Utilities|FlowControl|Delay 0.2)
          (Game|SpawnActorfromClass "/Game/Weapons/Projectiles/BP_Bullet_Master.BP_Bullet_Master_C" (Transformation|GetSocketTransform (Variables|Default|GetStaticMeshBarrelR) "FireSocket" "RTS_World") "Undefined" 0 0)
          (Components|Timeline|PlayfromStart (Variables|Default|GetRecoilTimelineR))
          (Utilities|FlowControl|Delay 0.2)
          (goto _label))))))

(event EventTick
  (params (DeltaSeconds :type Float%20%28single-precision%29))
  (Class|Turret|FindBestTarget)
  (Variables|Default|GetTarget
    (:then
      (Class|Turret|UpdateTurretRotation DeltaSeconds)
      (Class|Turret|UpdateFire))
    (:else)))

(fn ConstructionScript)